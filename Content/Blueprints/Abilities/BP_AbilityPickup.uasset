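; BP_AbilityPickup is an ability pickup actor that grants its AbilityType to a BP_Captain entering its PlayerCheck component.
; On overlap it sends an HTTP GET to a Supabase user-status table, using the captain's API key.
; The captain parses the JSON response, and the pickup loops over the records for hard-coded UserId 6.
; On a match it calls GainAbility with a zero recovery rate and destroys itself.
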(event OnComponentBeginOverlap(PlayerCheck)
  (params (OverlappedComponent :type Primitive%20Component%20Object%20Reference) (OtherActor :type Actor%20Object%20Reference) (OtherComp :type Primitive%20Component%20Object%20Reference) (OtherBodyIndex :type Integer) (bFromSweep :type Boolean) (SweepResult :type Hit%20Result%20Structure%20%28by%20ref%29))
  (bind _asbp_captain (Utilities|Casting|CastToBP_Captain OtherActor))
  (bind _result_body (|HttpRequest "https://heteivrmhzvvnyuaedny.supabase.co/rest/v1/DT_UserStatus" "Get" (|MakeRequestHeader "Custom" "apikey" (Variables|/Game/Blueprints/Characters/Captain/BP_Captain.BP_Captain_C|GetAPIKey _asbp_captain)))
    (:On%20Success
      (bind _resultfstructarray (Default|StatusJsontoFStructArray _asbp_captain _result_body))
      (for _array_element _resultfstructarray
        (Variables|Default|SetMyCharacterData _array_element)
        (if (== (.userid (Variables|Default|GetMyCharacterData)) 6)
          (Default|GainAbility _asbp_captain (Variables|Default|GetAbilityType) (/ 0 50))
          (Actor|DestroyActor))))))

(event EventBeginPlay)

(event Collision|EventActorBeginOverlap
  (params (OtherActor :type Actor%20Object%20Reference)))

(event EventTick
  (params (DeltaSeconds :type Float%20%28single-precision%29)))

(fn ConstructionScript)