(event EventBeginPlay
  (Variables|Default|SetGameTime 0.0)
  (Variables|Default|SetKilledShark 0))

(event EventTick
  (params (DeltaSeconds :type Float%20%28single-precision%29))
  (Variables|Default|SetGameTime (+ DeltaSeconds (Variables|Default|GetGameTime))))

(fn ConstructionScript)

(fn WinGame
  (bind _returnvalue (UserInterface|CreateWidget "/Game/Blueprints/Widgets/WBP_Score.WBP_Score_C"))
  (UserInterface|Viewport|AddtoViewport _returnvalue 0))

(fn DefeatGame
  (bind _returnvalue (UserInterface|CreateWidget "/Game/Blueprints/Widgets/WBP_YouDied.WBP_YouDied_C"))
  (UserInterface|Viewport|AddtoViewport _returnvalue 0)
  (UserInterface|Animation|PlayAnimation _returnvalue (Variables|/Game/Blueprints/Widgets/WBP_YouDied.WBP_YouDied_C|GetFadeIn _returnvalue) 0.0 1 "Forward" 1.0 false))

(fn QuitGame
  (Game|QuitGame 0 "Quit" false))

(fn RestartWidget
  (bind _returnvalue (UserInterface|CreateWidget "/Game/Blueprints/Widgets/WBP_MainPage.WBP_MainPage_C"))
  (UserInterface|Viewport|AddtoViewport _returnvalue 0))

(fn RestartGame
  (Game|OpenLevel(byName) "Demo"))