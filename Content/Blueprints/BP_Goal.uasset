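; BP_Goal is a level goal trigger that wins the game when a BP_Captain overlaps its box.
; After a short delay, a DoOnce makes the player's captain invincible, refills the overlapping captain's health and calls WinGame on GM_Action.
; Following a further delay, it calls RestartWidget on the game mode and opens the hard-coded Map_DEBUG level.
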(event OnComponentBeginOverlap(Box)
  (params (OverlappedComponent :type Primitive%20Component%20Object%20Reference) (OtherActor :type Actor%20Object%20Reference) (OtherComp :type Primitive%20Component%20Object%20Reference) (OtherBodyIndex :type Integer) (bFromSweep :type Boolean) (SweepResult :type Hit%20Result%20Structure%20%28by%20ref%29))
  (bind _asbp_captain (Utilities|Casting|CastToBP_Captain OtherActor))
  (Utilities|FlowControl|Delay 0.5)
  (Utilities|FlowControl|DoOnce false
    (:Completed
      (bind _asbp_captain_2 (Utilities|Casting|CastToBP_Captain (Game|Player|GetPlayerPawn 0)))
      (Variables|/Game/Blueprints/Characters/Captain/BP_Captain.BP_Captain_C|SetIsInvincibility _asbp_captain_2 true)
      (Variables|/Game/Blueprints/Characters/BP_ActionChar.BP_ActionChar_C|SetCurrentHealth _asbp_captain (Variables|/Game/Blueprints/Characters/BP_ActionChar.BP_ActionChar_C|GetMaxHealth _asbp_captain))
      (bind _asgm_action (Utilities|Casting|CastToGM_Action (Game|GetGameMode)))
      (Default|WinGame _asgm_action)
      (Utilities|FlowControl|Delay 4.0)
      (Default|RestartWidget _asgm_action)
      (Game|OpenLevel(byName) "Map_DEBUG"))))

(fn ConstructionScript)